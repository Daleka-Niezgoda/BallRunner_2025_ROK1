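; BP_TiltingPlatform_01 is a platform that rolls toward a tilt angle while the player's BP_Ball_01 pawn is on its collider.
; Overlap events set a tilting flag, though any actor ending overlap clears it.
; Tick interpolates roll toward the angle or back to level, tilting at a tenth of the return rate.
; It reads world roll but writes relative rotation, zeroing pitch and yaw.
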(event `self.Collider.OnComponentBeginOverlap`
  (params (OverlappedComponent :type "PrimitiveComponent Object Reference") (OtherActor :type "Actor Object Reference") (OtherComp :type "PrimitiveComponent Object Reference") (OtherBodyIndex :type Integer) (bFromSweep :type Boolean) (SweepResult :type "HitResult Structure (by ref)"))
  (bind _asbp_ball_01 (cast `/Game/BlueprintClasses/BP_Ball_01` (`GameplayStatics.GetPlayerPawn` 0)))
  (if (== _asbp_ball_01 OtherActor)
    (set `self.IsTilting` true)))

(event `self.Collider.OnComponentEndOverlap`
  (params (OverlappedComponent :type "PrimitiveComponent Object Reference") (OtherActor :type "Actor Object Reference") (OtherComp :type "PrimitiveComponent Object Reference") (OtherBodyIndex :type Integer))
  (set `self.IsTilting` false))

(event `self.ReceiveTick`
  (params (DeltaSeconds :type "Float (single-precision)"))
  (bind _platform (`self.platform`))
  (bind _tiltspeed (`self.TiltSpeed`))
  (bind _roll (.roll (`SceneComponent.K2_GetComponentRotation` (`self.platform`))))
  (if (`self.IsTilting`)
    (`SceneComponent.K2_SetRelativeRotation` _platform (`KismetMathLibrary.MakeRotator` (`KismetMathLibrary.FInterpTo` _roll (`self.TiltAngle`) (* DeltaSeconds 0.1) _tiltspeed)) true false)
    (else
      (`SceneComponent.K2_SetRelativeRotation` _platform (`KismetMathLibrary.MakeRotator` (`KismetMathLibrary.FInterpTo` _roll 0.0 DeltaSeconds _tiltspeed)) true false))))

(fn `UserConstructionScript`)